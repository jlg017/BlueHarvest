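; Base AI civilian character that tracks Food, Washroom and Entertainment stats.
; On possession by a civilian AI controller, it randomizes the stats and runs the BT_CivilianBase behavior tree.
; UseResource raises the chosen stat and lowers the others through a clamped 0-100 helper, then logs the use.
; The Food case computes its second value (the Washroom position) from Food instead of Washroom.
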(event `self.ReceivePossessed`
  (params (NewController :type "Controller Object Reference"))
  (bind _asbp_civilian_aicontroller (cast `/Game/AI/Controllers/BP_CivilianAIController` NewController))
  (set `self.AIController` _asbp_civilian_aicontroller)
  (`self.InitializeStats`)
  (`AIController.RunBehaviorTree` (`self.AIController`) "/Game/AI/Behaviours/Civilian/BT_CivilianBase.BT_CivilianBase"))

(fn `InitializeStats`
  (set `self.Stats` (make `/Game/AI/Behaviours/Civilian/S_CivilianStats` (`KismetMathLibrary.RandomInteger` 100) (`KismetMathLibrary.RandomInteger` 100) (`KismetMathLibrary.RandomInteger` 100))))

(fn `UpdateStatValue`
  (params (Value :type Integer) (DeltaValue :type Integer))
  (returns (NewValue :type Integer))
  (return (`KismetMathLibrary.Clamp` (+ Value DeltaValue) 0 100)))

(fn `UserConstructionScript`)

(fn `UseResource`
  (params (ResourceType :type "/Game/AI/SmartObjects/CivilianPOIs/E_ResourceType Enum" :default "NewEnumerator0"))
  (bind (_food _washroom _entertainment) (break `/Game/AI/Behaviours/Civilian/S_CivilianStats` (`self.Stats`)))
  (switch `/Game/AI/SmartObjects/CivilianPOIs/E_ResourceType` ResourceType
    (:`NewEnumerator0`
      (set `self.Stats` (make `/Game/AI/Behaviours/Civilian/S_CivilianStats` (`self.UpdateStatValue` _food 20) (`self.UpdateStatValue` _food -20) (`self.UpdateStatValue` _entertainment -20))))
    (:`NewEnumerator1`
      (set `self.Stats` (make `/Game/AI/Behaviours/Civilian/S_CivilianStats` (`self.UpdateStatValue` _food -20) (`self.UpdateStatValue` _washroom 20) (`self.UpdateStatValue` _entertainment -20))))
    (:`NewEnumerator2`
      (set `self.Stats` (make `/Game/AI/Behaviours/Civilian/S_CivilianStats` (`self.UpdateStatValue` _food -20) (`self.UpdateStatValue` _washroom -20) (`self.UpdateStatValue` _entertainment 20)))))
  (`KismetSystemLibrary.LogString` "Civilian used resource"))