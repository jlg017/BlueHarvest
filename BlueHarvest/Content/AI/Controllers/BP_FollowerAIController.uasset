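; AI controller for follower pawns that randomly swaps the character's visible mesh when its visible-to-player ID changes.
; On possess it caches the pawn as a BP_SingleVisibilityCharacter, logging an error if the cast fails.
; An ID-change handler bound at BeginPlay calls SetVisibleMesh with a random index; passing array length minus one to RandomInteger excludes the last mesh.
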(event `self.ReceiveBeginPlay`
  (add `self.OnVisibleToPlayerIdChanged` (delegate `HandleOnTargetIdChanged`)))

(event `HandleOnTargetIdChanged` :!signature `self.OnVisibleToPlayerIdChanged`
  (params (NewValue :type Integer))
  (`/Game/AI/Characters/BP_SingleVisibilityCharacter.SetVisibleMesh` (`self.SingleVisCharacter`) (`KismetMathLibrary.RandomInteger` (- (`KismetArrayLibrary.Array_Length` (`/Game/AI/Characters/BP_SingleVisibilityCharacter.Meshes` (`self.SingleVisCharacter`))) 1))))

(event `self.ReceivePossess`
  (params (PossessedPawn :type "Pawn Object Reference"))
  (bind _asbp_single_visibility_character (cast `/Game/AI/Characters/BP_SingleVisibilityCharacter` PossessedPawn)
    (:`then`
      (set `self.SingleVisCharacter` _asbp_single_visibility_character))
    (:`CastFailed`
      (`KismetSystemLibrary.LogString` "ERROR: Failed to cast controlled pawn to BP Single Visibility Character"))))

(fn `UserConstructionScript`)