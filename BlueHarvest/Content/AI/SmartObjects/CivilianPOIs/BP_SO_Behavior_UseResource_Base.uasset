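; Base smart object behavior for civilian AI points of interest where a character uses a resource.
; When triggered, it casts the avatar to the civilian base class and plays a montage on its skeletal mesh.
; Completion calls UseResource with the configured resource type, then ends the behavior; interruption ends it without using the resource.
; A failed cast logs an error and ends the behavior on the stored civilian reference, which that path never sets.
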(event `self.K2_OnTriggeredCharacter`
  (params (Avatar :type "Character Object Reference") (Config :type "GameplayBehaviorConfig Object Reference") (SmartObjectOwner :type "Actor Object Reference"))
  (bind _civiliancharacter (`self.CivilianCharacter`))
  (bind _asbp_aicivilian_character_base (cast `/Game/AI/Characters/BP_AICivilianCharacterBase` Avatar)
    (:`then`
      (set `self.CivilianCharacter` _asbp_aicivilian_character_base)
      (`|PlayMontage` (`Actor.GetComponentByClass` (`self.CivilianCharacter`) "/Script/Engine.SkeletalMeshComponent") (`self.AnimMontage`)
        (:`OnCompleted`
          (`/Game/AI/Characters/BP_AICivilianCharacterBase.UseResource` _civiliancharacter (`self.ResourceType`)))
        (:`OnInterrupted`
          _))
      (`self.K2_EndBehavior` _civiliancharacter))
    (:`CastFailed`
      (`KismetSystemLibrary.LogString` "Could not cast character to AI Civilian")
      (`self.K2_EndBehavior` (`self.CivilianCharacter`)))))