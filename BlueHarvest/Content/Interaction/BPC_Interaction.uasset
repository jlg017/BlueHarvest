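; Player interaction component that detects interactable actors in view and lets the player use them with E.
; Each tick, a short Visibility trace from player 0's camera finds BPI_Interaction actors and shows their interaction data in WB_Interaction, hiding it when the target is lost.
; Pressing E sends InteractMessage to the target locally, then again through the SR_Interact event, with an IsServer flag distinguishing the two calls.
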(event `self.ReceiveBeginPlay`
  (bind _widgetref (`/Game/Interaction/BML_ActorComponent.Get_WidgetReference` "/Game/Interaction/WB_Interaction.WB_Interaction_C")
    (:`true`
      (bind _aswb_interaction (cast `/Game/Interaction/WB_Interaction` _widgetref))
      (set `self.As WB Interaction` _aswb_interaction))))

(event `self.ReceiveTick`
  (params (DeltaSeconds :type "Float (single-precision)"))
  (`self.InteractionTrace` 250.0))

(event `Key|E`
  (params (Key :type "Key Structure"))
  (bind _returnvalue (`self.GetOwner`))
  (:`Pressed`
    (`self.InteractActor`
      (:`then`
        (message `/Game/Interaction/BPI_Interaction.Interact` (`self.InteractActor`) _returnvalue false)
        (`self.SR_Interact` (`self.InteractActor`) _returnvalue))
      (:`else`))))

(event `SR_Interact`
  (params (Target :type "Object Object Reference") (PlayerThatInteracts :type "Actor Object Reference"))
  (message `/Game/Interaction/BPI_Interaction.Interact` Target PlayerThatInteracts true))

(fn `InteractionTrace`
  (params (TraceLength :type "Float (single-precision)" :default 250.0))
  (bind _returnvalue (`GameplayStatics.GetPlayerCameraManager` 0))
  (bind _returnvalue_2 (`Actor.K2_GetActorLocation` _returnvalue))
  (bind (_outhit _returnvalue_3) (`KismetSystemLibrary.LineTraceSingle` _returnvalue_2 (+ _returnvalue_2 (* (`Actor.GetActorForwardVector` _returnvalue) TraceLength)) "TraceTypeQuery1"))
  (if _returnvalue_3
    (bind (_bblockinghit _binitialoverlap _time _distance _location _impactpoint _normal _impactnormal _physmat _hitactor) (`GameplayStatics.BreakHitResult` _outhit))
    (if (`KismetSystemLibrary.DoesImplementInterface` _hitactor "/Game/Interaction/BPI_Interaction.BPI_Interaction_C")
      (bind _output_get (set `self.InteractActor` _hitactor))
      (bind _interactiontext (message `/Game/Interaction/BPI_Interaction.Get_InteractData` _output_get))
      (`/Game/Interaction/WB_Interaction.Update_WBInteraction` (`self.As WB Interaction`) true _interactiontext)
      (else
        (`self.InteractActor` :!label _label
          (:`then`
            (set `self.InteractActor` null)
            (`/Game/Interaction/WB_Interaction.Update_WBInteraction` (`self.As WB Interaction`) false ""))
          (:`else`))))
    (else
      (goto _label))))