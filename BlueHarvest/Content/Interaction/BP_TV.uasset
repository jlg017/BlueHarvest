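; Interactable TV actor that swaps its static mesh when used.
; Interact branches on IsServer: true calls the MC_InteractionEvent (named as a multicast), false only calls PlaySoundAtLocation at the actor's location, with no sound asset shown.
; A FlipFlop in that event alternates the mesh between a bean bag and a 1970s vintage television, starting with the bean bag.
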(event `/Game/Interaction/BPI_Interaction.Interact`
  (params (PlayerThatInteracts :type "Actor Object Reference") (IsServer :type Boolean))
  (if IsServer
    (`self.MC_InteractionEvent`)
    (else
      (`GameplayStatics.PlaySoundAtLocation` null (`self.K2_GetActorLocation`) (struct) 1.0 1.0 0.0 null null null null))))

(event `MC_InteractionEvent`
  (`/Engine/EditorBlueprintResources/StandardMacros.FlipFlop`
    (:`A`
      (`StaticMeshComponent.SetStaticMesh` (`self.StaticMesh`) "/Game/Assets/Fab/Bean_Bag_-_Base_Mesh_2/bean_bag_base_mesh_2.bean_bag_base_mesh_2"))
    (:`B`
      (`StaticMeshComponent.SetStaticMesh` (`self.StaticMesh`) "/Game/Assets/Fab/1970_s__Vintage_Television/1970s_vintage_television.1970s_vintage_television"))))

(fn `UserConstructionScript`
  (`parent.UserConstructionScript`))