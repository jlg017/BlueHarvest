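; BP_LockableDoor is a networked interactable door that shows different prompt text when locked or unlocked.
; A server interaction toggles the replicated IsClosed if unlocked, and its RepNotify plays or reverses a timeline rotating the door pivot.
; A non-server interaction on a locked door spawns a lockpicking minigame actor below the door, whose OnLockPicked event clears IsLocked.
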(event `/Game/Interaction/BPI_Interaction.Interact`
  (params (PlayerThatInteracts :type "Actor Object Reference") (IsServer :type Boolean))
  (bind _islocked (`self.isLocked`))
  (if IsServer
    (if (not _islocked)
      (`self.SetIsClosed`))
    (elif _islocked
      (`self.PlayLockpickingMinigame`)
      (add `/Game/InteractiveObjects/Minigames/BP_LockpickingMinigame.OnLockPicked` (`self.LockPickingMinigame`) (delegate `OnLockPicked`)))))

(event `OnLockPicked`
  (set `self.isLocked` false))

(event `SetIsClosed`
  (set `self.isClosed` (not (`self.isClosed`))))

(event `BeginOpenDoor`
  (if (not (`self.isClosed`))
    (bind (_direction _doorrotationz) (`Timeline|OpenDoor` :!label _label)
      (:`Update`
        (`SceneComponent.K2_SetRelativeRotation` (`self.DoorPivot`) (`KismetMathLibrary.RotatorFromAxisAndAngle` (0.0 0.0 1.0) _doorrotationz) false false)))
    (else
      (goto _label :!via `Reverse`))))

(fn `Get_InteractData`
  (returns (InteractionText :type String))
  (if (`self.isLocked`)
    (return (`self.LockedInteractionText`))
    (else
      (return (`self.UnlockedInteractionText`)))))

(fn `OnRep_isClosed`
  (`self.BeginOpenDoor`))

(fn `OnRep_isLocked`)

(fn `PlayLockpickingMinigame`
  (bind _returnvalue (`|SpawnActorFromClass` "/Game/InteractiveObjects/Minigames/BP_LockpickingMinigame.BP_LockpickingMinigame_C" (`KismetMathLibrary.Conv_VectorToTransform` (+ (`self.K2_GetActorLocation`) (0.0 0.0 -1000.0))) "Undefined" "MultiplyWithRoot" null null))
  (set `self.LockPickingMinigame` _returnvalue))

(fn `UserConstructionScript`
  (`parent.UserConstructionScript`))