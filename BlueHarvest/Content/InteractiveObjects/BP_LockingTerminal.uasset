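; BP_LockingTerminal is an interactable terminal that gates its use behind a lockpicking minigame.
; On Interact, the server plays a timeline that moves the Base component if unlocked, while the non-server branch spawns BP_LockpickingMinigame far below the terminal if locked.
; A disconnected graph toggles IsLocked and plays or reverses a SolveAnimation, so nothing here unlocks it.
; GetInteractData supplies the interaction text.
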(event `/Game/Interaction/BPI_Interaction.Interact`
  (params (PlayerThatInteracts :type "Actor Object Reference") (IsServer :type Boolean))
  (bind _islocked (`self.isLocked`))
  (if IsServer
    (if (not _islocked)
      (bind (_direction _screenrotate) (`Timeline|Timeline`)
        (:`Update`
          (`SceneComponent.K2_SetRelativeLocation` (`self.Base`) _screenrotate false false))))
    (elif _islocked
      (bind _returnvalue (`|SpawnActorFromClass` "/Game/InteractiveObjects/Minigames/BP_LockpickingMinigame.BP_LockpickingMinigame_C" (`KismetMathLibrary.Conv_VectorToTransform` (+ (`self.K2_GetActorLocation`) (0.0 0.0 -1000.0))) "Undefined" "MultiplyWithRoot" null null))
      (set `self.LockPickingMinigame` _returnvalue))))

(fn `Get_InteractData`
  (returns (InteractionText :type String))
  (return (`self.Interaction Text_0`)))

(fn `UserConstructionScript`
  (`parent.UserConstructionScript`))