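; Lockpicking minigame actor where the player rotates a pick to find a randomly generated two-axis target.
; On BeginPlay it adds the lockpick widget, limits a scene capture to its own components, takes input from the character and randomizes the target.
; Tick turns the pick's clamped yaw and roll from axis input.
; When both fall within tolerance, it restores character input, removes the widget, destroys itself and calls OnLockPicked.
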(event `self.ReceiveBeginPlay`
  (bind _returnvalue (`GameplayStatics.GetPlayerController` 0))
  (bind _returnvalue_2 (`|CreateWidget` "/Game/InteractiveObjects/Minigames/WBP_LockPicking_Minigame.WBP_LockPicking_Minigame_C"))
  (bind _output_get (set `self.LockpickWidget` _returnvalue_2))
  (`UserWidget.AddToViewport` _output_get 0)
  (`SceneCaptureComponent.ShowOnlyActorComponents` (`self.SceneCaptureComponent2D`) self false)
  (`self.DisableInput` (`GameplayStatics.GetPlayerCharacter` 0) _returnvalue)
  (`self.EnableInput` _returnvalue)
  (`self.GenerateLock`))

(event `self.ReceiveTick`
  (params (DeltaSeconds :type "Float (single-precision)"))
  (bind _returnvalue (`GameplayStatics.GetPlayerController` 0))
  (bind _errortolerance (`self.ErrorTolerance`))
  (bind _lockminrot (`self.LockMinRot`))
  (bind _lockmaxrot (`self.LockMaxRot`))
  (bind (_relativerotation_roll _relativerotation_pitch _relativerotation_yaw) (`KismetMathLibrary.BreakRotator` (`SceneComponent.RelativeRotation` (`self.LeftPick_Scene`))))
  (bind (_relativerotation_roll_2 _relativerotation_pitch_2 _relativerotation_yaw_2) (`KismetMathLibrary.BreakRotator` (`SceneComponent.RelativeRotation` (`self.LeftPick_Scene`))))
  (`SceneComponent.K2_SetRelativeRotation` (`self.LeftPick_Scene`) (`KismetMathLibrary.MakeRotator` (`KismetMathLibrary.FClamp` (+ _relativerotation_roll_2 (* (`self.GetInputAxisKeyValue`) -0.1)) _lockminrot _lockmaxrot) 0.0 (`KismetMathLibrary.FClamp` (+ _relativerotation_yaw_2 (* (`self.GetInputAxisKeyValue`) -0.1)) _lockminrot _lockmaxrot)) false false)
  (if (and (`KismetMathLibrary.NearlyEqual_FloatFloat` (`self.LockY`) _relativerotation_roll _errortolerance) (`KismetMathLibrary.NearlyEqual_FloatFloat` _relativerotation_yaw (`self.LockX`) _errortolerance))
    (`self.DisableInput` _returnvalue)
    (`self.EnableInput` (`GameplayStatics.GetPlayerCharacter` 0) _returnvalue)
    (`Widget.RemoveFromParent` (`self.LockpickWidget`))
    (`self.K2_DestroyActor`)
    (`self.OnLockPicked`)))

(fn `GenerateLock`
  (bind _returnvalue (`KismetMathLibrary.RandomFloatInRange` (`self.LockMinRot`) (`self.LockMaxRot`)))
  (set `self.LockX` _returnvalue)
  (set `self.LockY` _returnvalue))

(fn `UserConstructionScript`)